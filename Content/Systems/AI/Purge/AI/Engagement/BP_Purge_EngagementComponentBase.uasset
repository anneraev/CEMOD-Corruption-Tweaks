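; Base engagement component for Purge attacker NPCs, steering whom they fight through the owner's TargetDistributionComponent.
; It registers as that component's DynamicEngagementBehavior and seeds distance-scaled hate on players and thrall defenders from the PurgeController.
; Locked doors trigger temporary building-attack hate, reverted when the door is destroyed or lost unless siege mode is active.
; Overridable queries define wanted targets, engagement filtering, treasure stealing and when carriers fight instead.
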(event Custom|Engage
  (params (IgnoreDistance :type Boolean))
  (bind _targetdistributioncomponent (Variables|Default|GetTargetDistributionComponent))
  (Variables|Default|GetPurgeController
    (:then
      (bind _targets (CallFunction|GatherEngagementTargets))
      (for _array_element _targets
        (if IgnoreDistance
          (Class|TargetDistributionComponent|AddHatetoTarget _targetdistributioncomponent (Utilities|Struct|MakeTargetWrapper _array_element -1) "InitialHate" (/ 1.0 (Transformation|GetHorizontalDistanceTo _array_element (Components|GetOwner)))) ; Unlimited range, add hate against EVERYTHING
          (elif (< (Transformation|GetHorizontalDistanceTo _array_element (Components|GetOwner)) 4e+03)
            (Class|TargetDistributionComponent|AddHatetoTarget _targetdistributioncomponent (Utilities|Struct|MakeTargetWrapper _array_element -1) "ProximityHate" (/ 4e+03 (Transformation|GetHorizontalDistanceTo _array_element (Components|GetOwner)))) ; Only hate targets within 40m, and scale by how close they are to me
          ))))
    (:else)))

(event Custom|OnTargetLost
  (params (Target :type Target%20Wrapper%20Structure%20%28by%20ref%29))
  (if (Math|Boolean|ANDBoolean (== (Utilities|ToObject(Interface) (.RawTarget (Utilities|Struct|BreakTargetWrapper Target))) (Variables|Default|GetDoorTarget)) (Utilities|IsValid (Variables|Default|GetDoorTarget)) (not (CallFunction|AttacksBuildings)))
    (CallFunction|RevertOutOfDoorAttackMode)))

(event Custom|ReachedTreasureRoom)

(event Custom|BindToDoorRelatedEvents
  (EventDispatchers|BindEventtoOnTargetLost (Variables|Default|GetTargetDistributionComponent) (delegate Custom|OnTargetLost)))

(event Custom|OnDoorTargetDestroyed
  (params (DestroyedActor :type Actor%20Object%20Reference))
  (if (and (== DestroyedActor (Variables|Default|GetDoorTarget)) (not (CallFunction|AttacksBuildings))) ; Door's open.  We can stop attacking buildings and go back to trying to steal treasure!
    (CallFunction|RevertOutOfDoorAttackMode)))

(event Custom|RevertOutOfDoorAttackMode
  (Utilities|FlowControl|Sequence
    (:then_0
      (bind _doortarget (Variables|Default|GetDoorTarget)
        (:then
          (Class|PlaceableBase|NPCDoneUsingNavLink _doortarget (.AsPawn (Utilities|Casting|CastToPawn (Components|GetOwner))))
          (Variables|Default|SetDoorTarget 0))
        (:else)))
    (:then_1
      (bind _asconan_character (Utilities|Casting|CastToConanCharacter (Components|GetOwner)))
      (Class|ConanCharacter|SetNPCAttacksBuildings _asconan_character false)
      (CallFunction|RemoveHateAgainstBuildings))))

(event Custom|EngageWithLockedDoor
  (params (Door :type Placeable%20Base%20Object%20Reference))
  (bind _targetwrapper (Utilities|Struct|MakeTargetWrapper Door -1))
  (bind _targetdistributioncomponent (Variables|Default|GetTargetDistributionComponent))
  (Variables|Default|SetDoorTarget Door)
  (bind _asconan_character (Utilities|Casting|CastToConanCharacter (Components|GetOwner)))
  (Class|ConanCharacter|SetNPCAttacksBuildings _asconan_character true)
  (Class|TargetDistributionComponent|AddHatetoTarget _targetdistributioncomponent _targetwrapper "InitialHateBuildings" 1e+04)
  (Class|TargetDistributionComponent|AddHatetoTarget _targetdistributioncomponent _targetwrapper "ProvokeHate" 5.0)
  (Game|BindEventtoOnDestroyed (Variables|Default|GetDoorTarget) (delegate Custom|OnDoorTargetDestroyed))
  (Class|PlaceableBase|NPCDoneUsingNavLink (Variables|Default|GetDoorTarget) (.AsConan%20Character (Utilities|Casting|CastToConanCharacter (Components|GetOwner)))) ; Don't leave the pathing nav component in an unresolved state.\nThe hate will take over on the next BT tick and the NPC will start attacking the door.
  (bind _returnvalue (AI|GetAIController (Components|GetOwner)))
  (AI|Components|Blackboard|SetValueasBool (AI|GetBlackboard _returnvalue) (Utilities|Name|MakeLiteralName "WillDefendInsteadOfCarrying") true) ; If carrying a treasure, make sure we *stop* carrying it and actually engage in combat
)

(event EventSetSiegeMode
  (params (Active :type Boolean))
  (Variables|Default|SetSiegeMode (Math|Boolean|NotEqual(Boolean) Active (Variables|Default|GetSiegeMode)))
  (bind _asconan_character (Utilities|Casting|CastToConanCharacter (Components|GetOwner)))
  (Class|ConanCharacter|SetNPCAttacksBuildings _asconan_character (Variables|Default|GetSiegeMode)))

(event EventBeginPlay
  (bind _output_get (Variables|Default|SetTargetDistributionComponent (Actor|GetComponentbyClass (Components|GetOwner) "/Script/ConanSandbox.TargetDistributionComponent")))
  (Utilities|IsValid _output_get
    (:Is%20Valid
      (Utilities|FlowControl|Sequence
        (:then_0
          (CallFunction|BindtoDoorRelatedEvents)
          (Variables|/Script/ConanSandbox.TargetDistributionComponent|SetDynamicEngagementBehavior (Variables|Default|GetTargetDistributionComponent) self)
          (if (Class|ActorComponent|IsComponentTickEnabled)
            (Class|ActorComponent|AddTickPrerequisiteComponent (Variables|Default|GetTargetDistributionComponent) self)
            (Class|ActorComponent|SetComponentTickInterval (Class|ActorComponent|GetComponentTickInterval (Variables|Default|GetTargetDistributionComponent)))))
        (:then_1
          (bind _returnvalue (AI|GetAIController (Components|GetOwner)))
          (bind _asconan_attacker_aicontroller (Utilities|Casting|CastToConanAttackerAIController _returnvalue))
          (Class|ConanAttackerAIController|SetShouldNotLeash _asconan_attacker_aicontroller true))))
    (:Is%20Not%20Valid
      (Components|DestroyComponent))))

(event EventEngagewithDoor
  (params (Placeable :type Placeable%20Base%20Object%20Reference))
  (bind _open (Class|DoorInterface|IsOpen(Message) Placeable))
  (if _open
    (Class|PlaceableBase|NPCDoneUsingNavLink Placeable (.AsPawn (Utilities|Casting|CastToPawn (Components|GetOwner))))
    (else
      (CallFunction|EngagewithLockedDoor Placeable))))

(fn FindMostHatedWantedTarget
  (for _array_element (Variables|/Script/ConanSandbox.TargetDistributionComponent|GetHateList (Variables|Default|GetTargetDistributionComponent))
    (if (CallFunction|IsWantedTarget (.Target (Utilities|Struct|BreakTargetData _array_element)))
      (if (> (Math|Float|Max(Float) (.Value (Utilities|Map|Find (.TotalHatePerTier (Utilities|Struct|BreakTargetData _array_element)) 0.0)) 1.0) (LocalVariables|GetLHateValue))
        (LocalVariables|SetLFoundTarget (.Target (Utilities|Struct|BreakTargetData _array_element)))
        (LocalVariables|SetLHateValue (Math|Float|Max(Float) (.Value (Utilities|Map|Find (.TotalHatePerTier (Utilities|Struct|BreakTargetData _array_element)) 0.0)) 1.0)))))
  (return (LocalVariables|GetLFoundTarget)))

(fn RemoveHatefromUnwantedTargets
  (params (InvertFilter :type Boolean))
  (LocalVariables|SetLInvert InvertFilter)
  (for _array_element (Variables|/Script/ConanSandbox.TargetDistributionComponent|GetHateList (Variables|Default|GetTargetDistributionComponent))
    (if (Class|KismetMathLibrary|XORBoolean (not (CallFunction|IsWantedTarget (.Target (Utilities|Struct|BreakTargetData _array_element)))) (LocalVariables|GetLInvert))
      (bind _enumvalue (|ForEachEHateType)
        (:LoopBody
          (if (Math|Boolean|ANDBoolean (Utilities|Enum|NotEqual(Enum) _enumvalue "OrderHate") (Utilities|Enum|NotEqual(Enum) _enumvalue "ProvokeHate") (Utilities|Enum|NotEqual(Enum) _enumvalue "TauntHate"))
            (Utilities|Map|Add (.CurrentHates (Utilities|Struct|BreakTargetData _array_element)) _enumvalue -1.0) ; If ALL hate values are <= 0, the target will be removed during the hatelist update
          ))))))

(fn PrioritizeSpecificTarget
  (params (Target :type Target%20Wrapper%20Structure))
  (Class|TargetDistributionComponent|AddHatetoTarget (Variables|Default|GetTargetDistributionComponent) Target "ProvokeHate" (* (Class|ActorComponent|GetComponentTickInterval) 2.0)))

(fn IsWantedTarget
  (params (Target :type Target%20Wrapper%20Structure))
  (return true))

(fn ShouldFightInsteadOfCarryingTreasure
  (bind _returnvalue (Components|GetOwner))
  (bind _asconan_character (Utilities|Casting|CastToConanCharacter _returnvalue))
  (bind _targetingcomponent (Variables|/Script/ConanSandbox.ConanCharacter|GetTargetingComponent _asconan_character))
  (bind (_outtarget _returnvalue_2) (Class|TargetDistributionComponent|GetTarget _targetingcomponent))
  (bind _rawtarget (Utilities|Struct|BreakTargetWrapper _outtarget))
  (if _returnvalue_2
    (Utilities|IsValid (Utilities|ToObject(Interface) _rawtarget)
      (:Is%20Valid
        (Utilities|Casting|CastToConanCharacter _rawtarget ; When the target is a character, only engage when we get low on HP\nWhen it's anything else, then immediately drop the treasure and engage (because it's probably a door/drawbridge blocking our path)
          (:then
            (return (< (CallFunction|GetCurrentHPRatio) 0.8)))
          (:CastFailed
            (return true))))
      (:Is%20Not%20Valid
        (return false)))
    (else
      (return false))))

(fn GetCurrentHPRatio
  (bind _asconan_character (Utilities|Casting|CastToConanCharacter (Components|GetOwner))
    (:then
      (return (/ (Math|Conversions|ToFloat(Integer) (Class|ConanCharacter|GetIntStat _asconan_character "HealthCurrent" "Full")) (Math|Conversions|ToFloat(Integer) (Class|ConanCharacter|GetIntStat _asconan_character "HealthMax" "Full")))))
    (:CastFailed
      (return 0.0))))

(fn GatherListOfTargetsfromPurgeController
  (params (IncludePlayers :type Boolean) (IncludeDefenders :type Boolean))
  (bind _purgecontroller (Variables|Default|GetPurgeController))
  (Utilities|FlowControl|Sequence
    (:then_0
      (if IncludePlayers
        (bind _returnvalue (Class|PurgeController|GetPlayerParticipants _purgecontroller))
        (Utilities|Array|AppendArray (LocalVariables|GetLTargets) _returnvalue)))
    (:then_1
      (if IncludeDefenders
        (bind _returnvalue_2 (Class|PurgeController|GetThrallDefenders _purgecontroller))
        (Utilities|Array|AppendArray (LocalVariables|GetLTargets) _returnvalue_2)))
    (:then_2
      (return (LocalVariables|GetLTargets)))))

(fn GatherEngagementTargets
  (bind _targets (CallFunction|GatherListOfTargetsfromPurgeController true true))
  (return _targets))

(fn IsPlayerSignificant
  (return false))

(fn IsTargetValid
  (params (Target :type Target%20Wrapper%20Structure))
  (Utilities|IsValidTarget Target
    (:Is%20Valid
      (return true))
    (:Is%20Not%20Valid
      (return false))))

(fn IsSpecialHateType
  (params (HateType :type EHateType%20Enum))
  (return (Utilities|Select :Index HateType :InitialHate true :InitialHateBuildings true :ProximityHate false :SenseHate false :SenseHateBuildings false :PhysicalHate false :TauntHate true :GiveUpHate true :LeashingHate true :OrderHate true :ProvokeHate false)))

(fn CanStealTreasure
  (return true))

(fn AttacksBuildings
  (return (Variables|Default|GetSiegeMode)))

(fn RemoveHateAgainstBuildings
  (bind _output_get (LocalVariables|SetLHateList (Variables|/Script/ConanSandbox.TargetDistributionComponent|GetHateList (Variables|Default|GetTargetDistributionComponent))))
  (for _array_element _output_get
    (Utilities|Casting|CastToConanCharacter (.RawTarget (Utilities|Struct|BreakTargetWrapper (.Target (Utilities|Struct|BreakTargetData _array_element))))
      (:CastFailed
        (bind _keys (Utilities|Map|Keys (.CurrentHates (Utilities|Struct|BreakTargetData _array_element))))
        (for _array_element_2 _keys
          (Class|TargetDistributionComponent|SetHateonTarget (Variables|Default|GetTargetDistributionComponent) (.Target (Utilities|Struct|BreakTargetData _array_element)) _array_element_2 0.0))))))

(fn IsWithinProxEngagementRange
  (params (Target :type Target%20Wrapper%20Structure))
  (bind _returnvalue (Components|GetOwner))
  (bind _asconan_character (Utilities|Casting|CastToConanCharacter _returnvalue))
  (bind _asconan_character_2 (Utilities|Casting|CastToConanCharacter (.RawTarget (Utilities|Struct|BreakTargetWrapper Target)))
    (:then
      (return (<= (- (- (Transformation|GetDistanceTo _asconan_character_2 _asconan_character) (.SphereRadius (Collision|GetComponentBounds (Class|ConanCharacter|GetCharacterCollision _asconan_character_2)))) (.SphereRadius (Collision|GetComponentBounds (Class|ConanCharacter|GetCharacterCollision _asconan_character)))) (Variables|Default|GetProximityEngagementRange))))
    (:CastFailed
      (return false))))

(fn CanEngageTarget
  (params (TargetDistributionComponent :type Target%20Distribution%20Component%20Object%20Reference) (Target :type Target%20Wrapper%20Structure%20%28by%20ref%29) (TriggeringHateType :type EHateType%20Enum :default "InitialHate"))
  (return (Math|Boolean|ORBoolean (CallFunction|IsWantedTarget Target) (CallFunction|IsWithinProxEngagementRange Target) (CallFunction|IsSpecialHateType TriggeringHateType))))

(fn ShouldOverrideCorpseDuration
  (return true 6e+01))