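; Sandstorm buff component that, on each tick, damages characters who are not sufficiently inside shelter, crediting a survival journey event instead if they wear sandstorm gear.
; Exposed ticks can also spawn hostile Kappa monsters, capped per player, using random ground traces ahead of the owner that accept only landscape hits.
; Spawns are aggroed on the owner; a timer culls targetless ones, and buff clear or owner destruction expires the rest at staggered times.
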(event Custom|StartMonsterTimer
  ;[1 1 1] Timed Check of monsters
  (Utilities|Time|SetTimerbyEvent (delegate Custom|ClearMonsters) 1e+01 true))

(event Custom|AttemptMonsterSpawn
  ;[1 1 1] Attempt Monster Spawn - chance check
  (if (>= (Math|Random|RandomIntegerinRange 1 100) 91)
    (CallFunction|SpawnMonster)))

(event Custom|SpawnMonster
  (bind _returnvalue (Components|GetOwner))
  (bind _returnvalue_2 (Math|Random|RandomFloatinRange 2.5e+02 5e+02))
  (bind _returnvalue_3 (Math|Random|RandomBool))
  (bind _returnvalue_4 (Transformation|GetActorForwardVector _returnvalue))
  (bind _returnvalue_5 (Transformation|GetActorLocation _returnvalue))
  (bind _returnvalue_6 (* _returnvalue_2 -1.0))
  (bind _returnvalue_7 (* _returnvalue_4 2.5e+03))
  (bind _returnvalue_8 (select _returnvalue_3 _returnvalue_6 _returnvalue_2))
  (bind _returnvalue_9 (+ _returnvalue_7 _returnvalue_5))
  (bind (_x _y _z) (Math|Vector|BreakVector _returnvalue_9))
  (bind _returnvalue_10 (+ _returnvalue_8 _y))
  (bind _returnvalue_11 (+ _returnvalue_2 _x))
  ;[1 1 1] Spawn Monster
  ;[1 1 1] Force an extra clearing of monsters if we spawn a monster
  (CallFunction|ClearMonsters)
  (if (not (Variables|Default|GetDEBUG_DisableMonsterSpawns))
    ;[1 1 1] Don't spawn more than 5 monsters per player
    (if (not (>= (Utilities|Array|Length (Variables|Default|GetMonsterArray)) 5))
      ;[1 1 1] Try a maximum of 5 linetraces
      (Variables|Default|SetLineTraceAttempts 0)
      ;[1 1 1] Attempt to find valid ground to spawn at
      (bind _outhit (Collision|LineTraceByChannel (Math|Vector|MakeVector _returnvalue_11 _returnvalue_10 _z) (Math|Vector|MakeVector _returnvalue_11 _returnvalue_10 -3e+04) "TraceTypeQuery6" false 0 "Persistent" :!label _label))
      (if (or (== (Utilities|GetClass (.HitActor (Collision|BreakHitResult _outhit))) "/Script/Landscape.Landscape") (Utilities|ClassIsChildOf (Utilities|GetClass (.HitActor (Collision|BreakHitResult _outhit))) "/Script/Landscape.LandscapeProxy"))
        ;[1 1 1] Spawn Monster, add to monsterarray, set navigation and roaming values. TODO: Spawn using tables, remove hardcoded stuff from here.
        (CallFunction|PlayParticletoHideMonsterSpawn (+ (.Location (Collision|BreakHitResult _outhit)) "0.0,0.0,100.000000"))
        (bind _returnvalue_12 (Class|FuncomGenericLibrary|LoadAssetfromPath "/Game/Systems/AI/BT_Attacker.BT_Attacker")) ; Asset by string to avoid confusing the blueprint compiler.
        (bind _asbehavior_tree (Utilities|Casting|CastToBehaviorTree _returnvalue_12))
        (bind _returnvalue_13 (Class|FuncomGenericLibrary|LoadClassfromPath "/Game/Characters/NPCs/Primates/Blueprints/BP_NPC_Wildlife_Kappa.BP_NPC_Wildlife_Kappa")) ; Asset by string to avoid confusing the blueprint compiler.
        (bind _aspawn (Utilities|Casting|CastToPawnClass _returnvalue_13))
        (bind (_success _npc) (CallFunction|TrySpawnNPCLowLevel _asbehavior_tree 0.0 _aspawn 0 (+ (.Location (Collision|BreakHitResult _outhit)) "0.0,0.0,100.000000") 2e+03 "Sandstorm spawning kappa: " 0 "" false "NewEnumerator3" false 0 0 0 0 0 0 "" "None"))
        (if _success
          (Utilities|Array|AddUnique (Variables|Default|GetMonsterArray) _npc)
          (bind _returnvalue_14 (AI|GetAIController _npc))
          (bind _asbp_aicontroller_character_interface (Utilities|Casting|CastToBP_AIControllerCharacterInterface _returnvalue_14))
          (Default|UpdateAttackerHate _asbp_aicontroller_character_interface (Components|GetOwner) 1e+02) ; Pretend player has been really nasty to this poor sandstorm monster.
        )
        (else
          (Math|Integer|IncrementInt (Variables|Default|GetLineTraceAttempts)
            (:%20%20
              (if (not (> (Variables|Default|GetLineTraceAttempts) 5))
                (goto _label)))))))))

(event Custom|KillAllMonsters
  ;[1 1 1] Remove all monsters by staggered timer
  (for _array_element (Variables|Default|GetMonsterArray)
    (Actor|SetLifeSpan _array_element (Math|Random|RandomFloatinRange 1.0 1e+01))))

(event Custom|ClearMonsters
  ;[1 1 1] Timed Check of monsters
  (for (_array_element _array_index) (Variables|Default|GetMonsterArray)
    (if (Utilities|IsValid _array_element)
      ;[1 1 1] Clears monsters without aggro
      (bind _returnvalue (AI|GetAIController _array_element))
      (bind _asbp_aicontroller_interface (Utilities|Casting|CastToBP_AIControllerInterface _returnvalue))
      (bind _hastarget (Default|HasTarget _asbp_aicontroller_interface))
      (if (not _hastarget)
        (Actor|DestroyActor _array_element)
        ;[1 1 1] Clears Dead Monsters
        (Utilities|Array|RemoveIndex (Variables|Default|GetMonsterArray) _array_index :!label _label))
      (else
        (goto _label)))))

(event Custom|OnDestroyed
  (params (DestroyedActor :type Actor%20Object%20Reference))
  ;[1 1 1] Start Monster Clearing Timer
  (CallFunction|KillAllMonsters))

(event Custom|PlayParticleToHideMonsterSpawn
  (params (Location :type Vector))
  ;[1 1 1] Particle to hide monster spawn
  (Effects|SpawnEmitteratLocation (Variables|Default|GetMonsterSpawnParticle) Location))

(event EventClientStartBuff
  (params (OwningCharacter :type Conan%20Character%20Object%20Reference) (Duration :type Float%20%28single-precision%29))
  (|CallParentFunction OwningCharacter Duration)
  (Variables|Default|SetInsideCheckerRef (Actor|GetComponentbyClass (Variables|Default|GetOwningCharacter) "/Game/Systems/Building/InsideChecker.InsideChecker_C")))

(event EventGameplayEffecttoApplyonBuffStart
  ;[1 1 1] Buff Start
  (|CallParentFunction)
  ;[1 1 1] Start Monster Clearing Timer
  (Game|AssignOnDestroyed (Components|GetOwner) (delegate Custom|OnDestroyed))
  (CallFunction|StartMonsterTimer))

(event EventGameplayEffecttoApplyonBuffTick
  (bind _insidecheckerref (Variables|Default|GetInsideCheckerRef))
  ;[1 1 1] Buff Tick
  (|CallParentFunction)
  ;[1 1 1] If True, then inside, do nothing
  (Utilities|IsValid _insidecheckerref
    (:Is%20Valid
      (if (not (>= (Variables|/Game/Systems/Building/InsideChecker.InsideChecker_C|GetInsidePercentage _insidecheckerref) 0.8))
        ;[1 1 1] Outside
        (CallFunction|AttemptMonsterSpawn :!label _label)
        ;;[1 1 1] Check if wearing mask
        (Utilities|IsValid (Actor|GetComponentbyClass (Variables|Default|GetOwningCharacter) "/Game/Systems/Buffs/Sandstorm/BP_AC_Sandstorm_Gear.BP_AC_Sandstorm_Gear_C")
          (:Is%20Valid
            (CallFunction|UpdateJourneyEvent))
          (:Is%20Not%20Valid
            (Game|Damage|ApplyDamage (Components|GetOwner) (* (Variables|Default|GetStackSize) (Variables|Default|GetDamagePerBuffTick)) (Pawn|GetController (Variables|Default|GetOwningCharacter)) (Variables|Default|GetDamageCauser) "/Game/Systems/Progression/DmgTypeHealth_BP_Landscape.DmgTypeHealth_BP_Landscape_C")))))
    (:Is%20Not%20Valid
      (goto _label))))

(event EventGameplayEffecttoApplyonBuffCleared
  ;[1 1 1] On Buff Cleared
  (|CallParentFunction)
  (CallFunction|KillAllMonsters))

(fn GetEffectDescription
  (bind _damageperbufftick (Variables|Default|GetDamagePerBuffTick))
  (bind _stacksize (Variables|Default|GetStackSize))
  (bind _bufftickduration (Variables|Default|GetBuffTickDuration))
  (bind _returnvalue (* _stacksize _damageperbufftick))
  (Utilities|IsValid (Variables|Default|GetInsideCheckerRef)
    (:Is%20Valid
      (if (>= (Variables|/Game/Systems/Building/InsideChecker.InsideChecker_C|GetInsidePercentage (Variables|Default|GetInsideCheckerRef)) 0.8)
        (if (>= (Utilities|Array|Length (Actor|GetComponentsByClass (Components|GetOwner) "/Game/Systems/Buffs/Sandstorm/BP_AC_Sandstorm_Gear.BP_AC_Sandstorm_Gear_C")) 1)
          (return (Utilities|Text|FormatText "Currently unaffected"))
          (else
            _)))
      (return (select (> (Math|Float|Truncate _returnvalue) 0) (Utilities|Text|FormatText "{TickDamage} points of damage every {TickTime}" (Math|Float|Truncate _returnvalue) (select (> _bufftickduration 1.0) (Utilities|Text|FormatText "{TickTime} seconds" _bufftickduration) "second")) "")))))

(fn UpdateJourneyEvent
  (if (Networking|IsServer)
    (bind _asbase_player_char_interface (Utilities|Casting|CastToBasePlayerCharInterface (Variables|Default|GetOwningCharacter)))
    (Default|AddJourneyEventInterfaceCall _asbase_player_char_interface "SurviveSandstorm")))